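; Demo actor that spins a mesh and orbits a Scene1 pivot while animating a dynamic material.
; Construction creates the material instance with initial color, texture and UV; BeginPlay starts a looping timer and a timeline driving UV's blue channel.
; ChangeColor randomly selects among three colors through a looping MultiGate.
; Tick applies delta-time rotations; both orbit and intended StaticMesh1 spin speeds rotate Scene1.
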(event Custom|ChangeColor
  (bind _mtd_staticmesh (Variables|Default|GetMTD_StaticMesh))
  (Utilities|FlowControl|MultiGate true true -1
    (:Out%200
      (Rendering|Material|SetVectorParameterValue _mtd_staticmesh "Color" "(R=1.000000,G=0.888101,B=0.364650,A=1.000000)" :!class /Script/Engine.MaterialInstanceDynamic))
    (:Out%201
      (Rendering|Material|SetVectorParameterValue _mtd_staticmesh "Color" "(R=0.177203,G=0.131958,B=1.000000,A=1.000000)" :!class /Script/Engine.MaterialInstanceDynamic))
    (:Out%202
      (Rendering|Material|SetVectorParameterValue _mtd_staticmesh "Color" "(R=0.297735,G=1.000000,B=0.463922,A=1.000000)" :!class /Script/Engine.MaterialInstanceDynamic))))

(event EventBeginPlay
  (Utilities|Time|SetTimerbyEvent 0 1.0 true)
  (bind _value (Timeline|UVTimeline Play)
    (:Update
      (bind _output_get (Variables|Default|SetUV (Utilities|Struct|MakeLinearColor (.r (Variables|Default|GetUV)) (.g (Variables|Default|GetUV)) _value (.a (Variables|Default|GetUV)))))
      (Rendering|Material|SetVectorParameterValue (Variables|Default|GetMTD_StaticMesh) "UV" _output_get :!class /Script/Engine.MaterialInstanceDynamic))))

(event EventTick
  (params (DeltaSeconds :type Float%20%28single-precision%29))
  (Utilities|FlowControl|Sequence
    (:then_0
      (Transformation|AddRelativeRotation (Variables|Default|GetStaticMesh) (Math|Rotator|MakeRotator 0.0 (* (Variables|Speed|GetstaticMeshLotationSpeed) DeltaSeconds) 0.0) false false))
    (:then_1
      ;[1 1 1] Static mesh rotateF Scene1 staticmesh1 공전
      (Transformation|AddRelativeRotation (Variables|Default|GetScene1) (Math|Rotator|MakeRotator 0.0 0.0 (* (Utilities|Time|GetWorldDeltaSeconds) (Variables|Speed|GetScene1LotationSpeed))) false false)
      ;[1 1 1] Static Mesh 1을 자전
      (Transformation|AddRelativeRotation (Variables|Default|GetScene1) (Math|Rotator|MakeRotator 0.0 0.0 (* (Utilities|Time|GetWorldDeltaSeconds) (Variables|Speed|GetstaticMesh1LotationSpeed))) false false))))

(fn ConstructionScript
  (bind _returnvalue (Rendering|Material|CreateDynamicMaterialInstance (Variables|Default|GetStaticMesh) 0 "/Game/Blueprint/MT_Textures.MT_Textures" "None" :!class /Script/Engine.PrimitiveComponent))
  (Utilities|IsValid _returnvalue
    (:Is%20Valid
      (bind _output_get (Variables|Default|SetMTD_StaticMesh _returnvalue))
      (Rendering|Material|SetVectorParameterValue _output_get "Color" (Variables|Default|GetValue) :!class /Script/Engine.MaterialInstanceDynamic)
      (Rendering|Material|SetTextureParameterValue _output_get "Texture" (Variables|Default|GetTexture))
      (Rendering|Material|SetVectorParameterValue (Variables|Default|GetMTD_StaticMesh) "UV" (Variables|Default|GetUV) :!class /Script/Engine.MaterialInstanceDynamic))))