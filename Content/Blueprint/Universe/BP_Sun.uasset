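; BP_Sun is a sun actor for a universe scene that spins, carries an orbit pivot and animates its glow.
; Tick rotates the root for the sun's spin and EarthAxis for orbital revolution, both at constant yaw rates scaled by delta time.
; The construction script creates a dynamic material on the mesh.
; On BeginPlay, the SunShine timeline plays at half speed, driving that material's Shining parameter.
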(event EventBeginPlay
  (Components|Timeline|SetPlayRate (Variables|Default|GetSunShine) 0.5)
  (bind _shining (Timeline|SunShine Play)
    (:Update
      (Rendering|Material|SetScalarParameterValue (Variables|Default|GetMID_Sun) "Shining" (* _shining 5e+01) :!class /Script/Engine.MaterialInstanceDynamic))))

(event Collision|EventActorBeginOverlap
  (params (OtherActor :type Actor%20Object%20Reference)))

(event EventTick
  (params (DeltaSeconds :type Float%20%28single-precision%29))
  (Utilities|FlowControl|Sequence
    (:then_0
      ;[1 1 1] 공전
      (Transformation|AddLocalRotation (Variables|Default|GetEarthAxis) (Math|Rotator|MakeRotator 0.0 0.0 (* 36.0 DeltaSeconds)) false false))
    (:then_1
      ;[1 1 1] 자전
      (Transformation|AddLocalRotation (Variables|Default|GetDefaultSceneRoot) (Math|Rotator|MakeRotator 0.0 0.0 (* 1e+01 DeltaSeconds)) false false))))

(fn ConstructionScript
  (bind _staticmesh (Variables|Default|GetStaticMesh))
  (bind _returnvalue (Rendering|Material|CreateDynamicMaterialInstance _staticmesh 0 (Rendering|Material|GetMaterial _staticmesh 0) "None" :!class /Script/Engine.PrimitiveComponent))
  (Variables|Default|SetMID_Sun _returnvalue))