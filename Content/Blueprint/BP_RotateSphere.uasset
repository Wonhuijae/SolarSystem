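; BP_RotateSphere is an actor that spins a mesh and turns a pivot, Scene1, to simulate self-rotation and orbit.
; Each Tick pitches StaticMesh and yaws Scene1 at variable-driven speeds scaled by delta time.
; The step commented as StaticMesh1's own spin also rotates Scene1, so both yaw speeds add on that pivot.
; BeginPlay prints a "Hello" debug string.
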(event EventBeginPlay
  (Development|PrintString "Hello"))

(event Collision|EventActorBeginOverlap
  (params (OtherActor :type Actor%20Object%20Reference)))

(event EventTick
  (params (DeltaSeconds :type Float%20%28single-precision%29))
  (Utilities|FlowControl|Sequence
    (:then_0
      (Transformation|AddRelativeRotation (Variables|Default|GetStaticMesh) (Math|Rotator|MakeRotator 0.0 (* (Variables|Speed|GetstaticMeshLotationSpeed) DeltaSeconds) 0.0) false false))
    (:then_1
      ;[1 1 1] Static mesh rotateF Scene1 staticmesh1 공전
      (Transformation|AddRelativeRotation (Variables|Default|GetScene1) (Math|Rotator|MakeRotator 0.0 0.0 (* (Utilities|Time|GetWorldDeltaSeconds) (Variables|Speed|GetScene1LotationSpeed))) false false)
      ;[1 1 1] Static Mesh 1을 자전
      (Transformation|AddRelativeRotation (Variables|Default|GetScene1) (Math|Rotator|MakeRotator 0.0 0.0 (* (Utilities|Time|GetWorldDeltaSeconds) (Variables|Speed|GetstaticMesh1LotationSpeed))) false false))))

(fn ConstructionScript)